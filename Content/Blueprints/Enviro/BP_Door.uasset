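; BP_Door is an environment door that opens once its activation count reaches the required number of locks.
; Each CEEnviroActivated call increments the count and, at or above the threshold, starts a looping timer at the frame delta in place of Tick.
; CE_Open slides the Cube along a Spline by normalized elapsed time over the open duration.
; At the end it empties the timer handle before the clear call, so that clear misses the running timer.
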(event `self.ReceiveTick`
  (params (DeltaSeconds :type "Float (single-precision)")))

(event `self.CE_EnviroActivated`
  (set `self.i_NumOfLock` (+ (`self.i_NumOfLock`) 1))
  (if (>= (`self.i_NumOfLock`) (`self.i_MaxLock`))
    (bind _returnvalue (`KismetSystemLibrary.K2_SetTimerDelegate` (delegate `CE_Open`) (`GameplayStatics.GetWorldDeltaSeconds`) true))
    (set `self.TH` _returnvalue)))

(event `CE_Open`
  (if (< (`self.f_CurrentTime`) (`self.f_OpenDuration`))
    (set `self.f_CurrentTime` (+ (`self.f_CurrentTime`) (`GameplayStatics.GetWorldDeltaSeconds`)))
    (set `self.f_Alpha` (`KismetMathLibrary.NormalizeToRange` (`self.f_CurrentTime`) 0.0 (`self.f_OpenDuration`)))
    (`SceneComponent.K2_SetWorldLocation` (`self.Cube`) (`SplineComponent.GetLocationAtTime` (`self.Spline`) (`self.f_Alpha`) "World" false) false false)
    (else
      (bind _output_get (set `self.TH` (struct)))
      (`KismetSystemLibrary.K2_ClearAndInvalidateTimerHandle` _output_get))))

(fn `UserConstructionScript`
  (`parent.UserConstructionScript`))