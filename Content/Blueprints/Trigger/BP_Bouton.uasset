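; BP_Bouton is an interactable toggle button trigger that switches on or off each time an interact input starts.
; Both transitions update the switch, call CEActiveAll, and refresh the cube's material to green when on or red when off.
; Turning it on also tells the BP_Mimic actor found at BeginPlay to check the button count.
; The construction script runs the same feedback so the color matches the initial state.
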(event `self.ReceiveBeginPlay`
  (bind _returnvalue (`GameplayStatics.GetActorOfClass` "/Game/Blueprints/AI/BP_Mimic.BP_Mimic_C"))
  (set `self.BP_Mimic` _returnvalue))

(event `self.CE_InteractInput`
  (params (E_InputState :type "/Game/FirstPerson/Input/E_InputState Enum" :default "NewEnumerator0"))
  (`parent.CE_InteractInput` E_InputState)
  (switch `/Game/FirstPerson/Input/E_InputState` (`self.E Input State`)
    (:`NewEnumerator1`
      (if (`self.b_IsOn`)
        (`self.CE_TriggerDesactivated`)
        (else
          (`self.CE_TriggerActivated`))))))

(event `self.CE_TriggerActivated`
  (set `self.b_IsOn` true)
  (`self.CE_SetActivatedSwitch` true)
  (`self.CE_ActiveAll`)
  (`self.CE_feedback`)
  (`/Game/Blueprints/AI/BP_Mimic.CE_CheckNumButton` (`self.BP_Mimic`)))

(event `CE_feedback`
  (`PrimitiveComponent.SetMaterial` (`self.Cube`) 0 (select `bool` (`self.b_IsOn`) :`false` "/Game/Enviro/Materials/MI_Red.MI_Red" :`true` "/Game/Enviro/Materials/MI_Green.MI_Green" :!type "MaterialInterface Object Reference")))

(event `self.CE_TriggerDesactivated`
  (set `self.b_IsOn` false)
  (`self.CE_SetActivatedSwitch` true)
  (`self.CE_ActiveAll`)
  (`self.CE_feedback`))

(fn `UserConstructionScript`
  (`self.CE_feedback`))