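; Base interactable trigger Blueprint that switches linked environment actors between activated and deactivated.
; Custom events store the interact input state and the activation switch.
; CE_ForEach loops over the ActorLink array and calls each actor's activate or deactivate event based on that switch.
; The trigger activated and deactivated events are placeholders, with only a debug print on activation, and nothing in this graph calls CE_ForEach.
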(event `CE_InteractInput`
  (params (E_InputState :type "/Game/FirstPerson/Input/E_InputState Enum" :default "NewEnumerator0"))
  (set `self.E Input State` E_InputState))

(event `CE_TriggerActivated`
  (`KismetSystemLibrary.PrintString` "Hello"))

(event `CE_TriggerDesactivated`)

(event `CE_ForEach`
  (for _array_element (`self.ActorLink`)
    (if (`self.b_ActivatedSwitch`)
      (`/Game/Blueprints/Enviro/BP_MainEnviro.CE_EnviroActivated` _array_element)
      (else
        (`/Game/Blueprints/Enviro/BP_MainEnviro.CE_EnviroDesactivated` _array_element)))))

(event `CE_SetActivatedSwitch`
  (params (b_ActivatedSwitch :type Boolean))
  (set `self.b_ActivatedSwitch` b_ActivatedSwitch))

(fn `UserConstructionScript`)