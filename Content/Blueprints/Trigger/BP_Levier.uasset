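; Lever trigger that the player holds interact on to fill a timed gauge, firing its linked activation once full.
; While held, it disables player movement, clamps the camera around the lever, and drives handle rotation and a material Alpha from progress.
; Pressing summons the Mimic to the lever in berserk mode.
; Release restores control, and a gated retriggerable delay ends berserk unless interaction restarts; gauge progress is kept.
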(event `self.ReceiveBeginPlay`
  (bind _asbp_player_character (cast `/Game/Blueprints/Player/BP_PlayerCharacter` (`GameplayStatics.GetPlayerCharacter` 0)))
  (set `self.As BP Player Character` _asbp_player_character)
  (bind _returnvalue (`GameplayStatics.GetActorOfClass` "/Game/Blueprints/AI/BP_Mimic.BP_Mimic_C"))
  (set `self.BP_Mimic` _returnvalue))

(event `self.CE_InteractInput`
  (params (E_InputState :type "/Game/FirstPerson/Input/E_InputState Enum" :default "NewEnumerator0"))
  (`parent.CE_InteractInput` E_InputState)
  (switch `/Game/FirstPerson/Input/E_InputState` (`self.E Input State`)
    (:`NewEnumerator0`
      (`self.CE_TriggerActivated` :!label _label))
    (:`NewEnumerator1`
      (`self.CE_CallMimic`)
      (`/Game/Blueprints/AI/BP_Mimic.CE_SetBerserk` (`self.BP_Mimic`) true)
      (goto _label_3 :!via `Close`))
    (:`NewEnumerator2`
      (goto _label))
    (:`NewEnumerator3`
      (`self.CE_TriggerDesactivated` :!label _label_2)
      (`KismetSystemLibrary.PrintString` "Hello")
      (`|ExecutionSequence`
        (:`then_0`
          (`KismetSystemLibrary.RetriggerableDelay` 3.0)
          (`/Engine/EditorBlueprintResources/StandardMacros.Gate` false :!label _label_3
            (:`Exit`
              (`/Game/Blueprints/AI/BP_Mimic.CE_SetBerserk` (`self.BP_Mimic`) false))))
        (:`then_1`
          (goto _label_3 :!via `Open`))))
    (:`NewEnumerator4`
      (goto _label_2))))

(event `self.CE_TriggerActivated`
  (`self.CE_AddGauge`)
  (`self.CE_LockMovement`))

(event `CE_LockMovement`
  (`CharacterMovementComponent.DisableMovement` (`Character.CharacterMovement` (`self.As BP Player Character`)))
  (`/Game/Blueprints/Player/BP_PlayerCharacter.CE_InteractPrio` (`self.As BP Player Character`) self)
  (`self.CE_Focus` true))

(event `self.CE_TriggerDesactivated`
  (`self.CE_DelockMovement`))

(event `CE_DelockMovement`
  (`CharacterMovementComponent.SetMovementMode` (`Character.CharacterMovement` (`self.As BP Player Character`)) "MOVE_Walking" 0)
  (`self.CE_Focus` false)
  (`/Game/Blueprints/Player/BP_PlayerCharacter.CE_InteractPrio` (`self.As BP Player Character`) null))

(event `CE_Focus`
  (params (`B Is Focus?` :type Boolean))
  (set `self.B Is Focus?` `B Is Focus?`)
  (`|ExecutionSequence`
    (:`then_0`
      (set `PlayerCameraManager.ViewPitchMin` (select `bool` (`self.B Is Focus?`) :`false` -90.0 :`true` (`KismetMathLibrary.FClamp` (- (`self.FC_GetCameraRot`) (`self.f_FocusAngle`)) -75.0 90.0) :!type "Float (single-precision)") (`GameplayStatics.GetPlayerCameraManager` 0)))
    (:`then_1`
      (set `PlayerCameraManager.ViewPitchMax` (select `bool` (`self.B Is Focus?`) :`false` 90.0 :`true` (+ (`self.FC_GetCameraRot`) (`self.f_FocusAngle`)) :!type "Float (single-precision)") (`GameplayStatics.GetPlayerCameraManager` 0)))
    (:`then_2`
      (set `PlayerCameraManager.ViewYawMin` (select `bool` (`self.B Is Focus?`) :`true` (- (`.ReturnValue_Yaw` (`self.FC_GetCameraRot`)) (`self.f_FocusAngle`)) :!type "Float (single-precision)") (`GameplayStatics.GetPlayerCameraManager` 0)))
    (:`then_3`
      (set `PlayerCameraManager.ViewYawMax` (select `bool` (`self.B Is Focus?`) :`false` 359.0 :`true` (+ (`.ReturnValue_Yaw` (`self.FC_GetCameraRot`)) (`self.f_FocusAngle`))) (`GameplayStatics.GetPlayerCameraManager` 0)))))

(event `CE_Feedback`
  (bind _sphere (`self.Sphere`))
  (`SceneComponent.K2_SetWorldRotation` (`self.Cube`) (`KismetMathLibrary.RLerp` (`KismetMathLibrary.FindLookAtRotation` (`SceneComponent.K2_GetComponentLocation` (`self.Cube`)) (`SceneComponent.K2_GetComponentLocation` (`self.TopSocket`))) (`KismetMathLibrary.FindLookAtRotation` (`SceneComponent.K2_GetComponentLocation` (`self.Cube`)) (`SceneComponent.K2_GetComponentLocation` (`self.BotSocket`))) (`self.f_Alpha`)) false false)
  (bind _returnvalue (`PrimitiveComponent.CreateDynamicMaterialInstance` _sphere 0 (`PrimitiveComponent.GetMaterial` _sphere 0) "None"))
  (`MaterialInstanceDynamic.SetScalarParameterValue` _returnvalue "Alpha" (`self.f_Alpha`)))

(event `CE_AddGauge`
  (if (< (`self.f_Gauge`) (`self.f_PushDuration`))
    (set `self.f_Gauge` (+ (`self.f_Gauge`) (`GameplayStatics.GetWorldDeltaSeconds`)))
    (set `self.f_Alpha` (`KismetMathLibrary.NormalizeToRange` (`self.f_Gauge`) 0.0 (`self.f_PushDuration`)))
    (`self.CE_Feedback`)
    (else
      (`self.CE_GaugeFull`))))

(event `CE_GaugeFull`
  (`/Engine/EditorBlueprintResources/StandardMacros.DoOnce` false
    (:`Completed`
      (`self.CE_SetActivatedSwitch` true)
      (`self.CE_ActiveAll`))))

(event `CE_CallMimic`
  (`/Game/Blueprints/AI/BP_Mimic.CE_MoveToObjectif` (`self.BP_Mimic`) self))

(fn `FC_GetCameraRot`
  (returns (ReturnValue_Pitch :type "Float (single-precision)") (ReturnValue_Yaw :type "Float (single-precision)"))
  (bind (_returnvalue_roll _returnvalue_pitch _returnvalue_yaw) (`KismetMathLibrary.BreakRotator` (`KismetMathLibrary.FindLookAtRotation` (`SceneComponent.K2_GetComponentLocation` (`/Game/Blueprints/Player/BP_PlayerCharacter.FirstPersonCamera` (`self.As BP Player Character`))) (`SceneComponent.K2_GetComponentLocation` (`self.Cube`)))))
  (return _returnvalue_pitch _returnvalue_yaw))

(fn `UserConstructionScript`
  (`parent.UserConstructionScript`))