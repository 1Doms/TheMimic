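; BP_Enviro is an environment actor that lays out copies of a configurable mesh in a flat X/Y grid.
; Its construction script assigns NewMesh to an InstancedStaticMesh component, then nested loops add instances using count variables and 128-unit spacing multiplied by per-axis scale variables.
; The outer loop also adds an instance per column, duplicating the inner loop's Y=0 instance.
; The event graph holds only disabled placeholder events.
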(fn `UserConstructionScript`
  (`StaticMeshComponent.SetStaticMesh` (`self.InstancedStaticMesh`) (`self.New Mesh`))
  (for _index (range (`self.i_Xnum`))
    (bind _returnvalue (`KismetMathLibrary.Conv_IntToDouble` (* _index (* (`self.i_Xscale`) 128))))
    (`InstancedStaticMeshComponent.AddInstance` (`self.InstancedStaticMesh`) (`KismetMathLibrary.MakeTransform` (`KismetMathLibrary.MakeVector` _returnvalue)) false)
    (for _index_2 (range (`self.i_Ynum`))
      (`InstancedStaticMeshComponent.AddInstance` (`self.InstancedStaticMesh`) (`KismetMathLibrary.MakeTransform` (`KismetMathLibrary.MakeVector` _returnvalue (`KismetMathLibrary.Conv_IntToDouble` (* _index_2 (* (`self.i_Yscale`) 128))))) false))))